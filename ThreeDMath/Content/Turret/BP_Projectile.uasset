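; A turret projectile actor that flies straight forward and disappears on contact.
; On BeginPlay it sets its ProjectileMovement max speed and local-space velocity from a NewSpeed variable.
; Any overlap on its Sphere1 component destroys the actor, with no damage or effects applied.
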(event OnComponentBeginOverlap(Sphere1)
  (params (OverlappedComponent :type Primitive%20Component%20Object%20Reference) (OtherActor :type Actor%20Object%20Reference) (OtherComp :type Primitive%20Component%20Object%20Reference) (OtherBodyIndex :type Integer) (bFromSweep :type Boolean) (SweepResult :type Hit%20Result%20Structure%20%28by%20ref%29))
  (Actor|DestroyActor))

(event EventBeginPlay
  (bind _projectilemovement (Variables|Default|GetProjectileMovement))
  (bind _newspeed (Variables|Default|GetNewSpeed))
  (Variables|/Script/Engine.ProjectileMovementComponent|SetMaxSpeed _projectilemovement _newspeed)
  (Game|Components|ProjectileMovement|SetVelocityinLocalSpace _projectilemovement (* (Class|KismetMathLibrary|VectorForward) _newspeed)))

(event EventTick
  (params (DeltaSeconds :type Float%20%28single-precision%29)))

(fn ConstructionScript)