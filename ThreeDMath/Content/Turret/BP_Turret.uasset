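; Turret that fires projectiles on a looping timer, leading a moving target that defaults to the player pawn.
; Tick derives target velocity from position deltas, while TurretConfig supplies projectile class, speed and fire interval.
; UseQuadratic selects either a closed-form intercept (CalculateShot) or an iterative travel-time search (PredictShot) to aim each shot and rotate the Sphere.
; PredictTargetPosition is an unused stub that returns the target's current location.
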(event Custom|Fire
  (bind _turretconfig (Variables|Default|GetTurretConfig))
  (bind _turretconfig_2 (Variables|Default|GetTurretConfig))
  (bind _barrel (Variables|Default|GetBarrel))
  (bind _barrel_2 (Variables|Default|GetBarrel))
  (bind _returnvalue (Transformation|GetWorldLocation _barrel))
  (bind _returnvalue_2 (Transformation|GetWorldLocation _barrel_2))
  (if (Variables|Default|GetbUseQuadratic)
    (bind _impactlocation (CallFunction|CalculateShot (Transformation|GetWorldLocation (Variables|Default|GetBarrel)) (Variables|/Game/Turret/BP_TurretConfig.BP_TurretConfig_C|GetProjectileSpeed (Variables|Default|GetTurretConfig)) (Transformation|GetActorLocation (Variables|Default|GetTarget)) (Variables|Default|GetTrackedTargetVelocity)))
    (Game|SpawnActorfromClass (Variables|/Game/Turret/BP_TurretConfig.BP_TurretConfig_C|GetProjectileClass _turretconfig_2) (Math|Transform|MakeTransform _returnvalue (Math|Rotator|FindLookatRotation _returnvalue _impactlocation) "1,1,1") "Undefined" 0 (Variables|/Game/Turret/BP_TurretConfig.BP_TurretConfig_C|GetProjectileSpeed _turretconfig_2) 0)
    (Transformation|SetWorldRotation (Variables|Default|GetSphere) (Math|Rotator|FindLookatRotation _returnvalue _impactlocation) false false)
    (else
      (bind _impactlocation_2 (CallFunction|PredictShot (Transformation|GetWorldLocation (Variables|Default|GetBarrel)) (Variables|/Game/Turret/BP_TurretConfig.BP_TurretConfig_C|GetProjectileSpeed (Variables|Default|GetTurretConfig)) (Variables|Default|GetTrackedTargetVelocity) (Transformation|GetActorLocation (Variables|Default|GetTarget)) 10))
      (Game|SpawnActorfromClass (Variables|/Game/Turret/BP_TurretConfig.BP_TurretConfig_C|GetProjectileClass _turretconfig) (Math|Transform|MakeTransform _returnvalue_2 (Math|Rotator|FindLookatRotation _returnvalue_2 _impactlocation_2) "1,1,1") "Undefined" 0 (Variables|/Game/Turret/BP_TurretConfig.BP_TurretConfig_C|GetProjectileSpeed _turretconfig) 0)
      (Transformation|SetWorldRotation (Variables|Default|GetSphere) (Math|Rotator|FindLookatRotation _returnvalue_2 _impactlocation_2) false false))))

(event Custom|CalculateTargetDelta
  (params (dt :type Float%20%28single-precision%29))
  (bind _velocity (CallFunction|TrackObjectVelocity (Transformation|GetActorLocation (Variables|Default|GetTarget)) (Variables|Default|GetLastTargetLocation) dt))
  (Variables|Default|SetTrackedTargetVelocity _velocity)
  (Variables|Default|SetLastTargetLocation (Transformation|GetActorLocation (Variables|Default|GetTarget))))

(event EventTick
  (params (DeltaSeconds :type Float%20%28single-precision%29))
  (CallFunction|CalculateTargetDelta DeltaSeconds))

(event Collision|EventActorBeginOverlap
  (params (OtherActor :type Actor%20Object%20Reference)))

(event EventBeginPlay
  (bind _returnvalue (Game|Player|GetPlayerPawn 0))
  (Utilities|IsValid (Variables|Default|GetTarget)
    (:Is%20Valid
      (Utilities|Time|SetTimerbyEvent (delegate Custom|Fire) (Variables|/Game/Turret/BP_TurretConfig.BP_TurretConfig_C|GetTimeBetweenShots (Variables|Default|GetTurretConfig)) true 2.0 1.0 :!label _label))
    (:Is%20Not%20Valid
      (Utilities|IsValid _returnvalue
        (:Is%20Valid
          (Variables|Default|SetTarget _returnvalue)
          (goto _label))
        (:Is%20Not%20Valid
          (Development|PrintString "No Target for turret" true true "(R=1.000000,G=0.451018,B=0.000000,A=1.000000)"))))))

(fn ConstructionScript)

(fn PredictTargetPosition
  (params (Target :type Actor%20Object%20Reference) (Projectile%20Velocity :type Float%20%28single-precision%29) (Iterations :type Integer))
  (LocalVariables|SetTargetLocation (Transformation|GetActorLocation Target)))

(fn TravelTime
  (params (V :type Float%20%28single-precision%29) (A :type Vector) (B :type Vector))
  (return (/ (Math|Vector|Distance(Vector) A B) V)))

(fn PostionAfterTime
  (params (T :type Float%20%28single-precision%29) (Pos :type Vector) (Vel :type Vector))
  (return (+ Pos (* Vel T))))

(fn PredictShot
  (params (Origin :type Vector) (BulletVelocity :type Float%20%28single-precision%29) (Velocity :type Vector) (Target :type Vector) (Iterations :type Integer))
  (bind _outeriterations (LocalVariables|GetOuterIterations))
  (LocalVariables|SetBestLocation Target)
  (LocalVariables|SetEstimatedTime (CallFunction|TravelTime BulletVelocity Origin Target))
  (for _index (range 0 _outeriterations)
    (for _index_2 (range 0 Iterations)
      (if (< (Math|Float|Absolute(Float) (- (CallFunction|TravelTime BulletVelocity Origin (+ Target (* Velocity (* (Math|Float|Lerp (- 1.0 (* (Math|Float|MakeLiteralFloat 1.5) (- 1.0 (/ (Math|Conversions|ToFloat(Integer) _index) (Math|Conversions|ToFloat(Integer) _outeriterations))))) (+ 1.0 (* (Math|Float|MakeLiteralFloat 1.5) (- 1.0 (/ (Math|Conversions|ToFloat(Integer) _index) (Math|Conversions|ToFloat(Integer) _outeriterations))))) (/ (Math|Conversions|ToFloat(Integer) _index_2) (Math|Conversions|ToFloat(Integer) Iterations))) (LocalVariables|GetEstimatedTime))))) (* (Math|Float|Lerp (- 1.0 (* (Math|Float|MakeLiteralFloat 1.5) (- 1.0 (/ (Math|Conversions|ToFloat(Integer) _index) (Math|Conversions|ToFloat(Integer) _outeriterations))))) (+ 1.0 (* (Math|Float|MakeLiteralFloat 1.5) (- 1.0 (/ (Math|Conversions|ToFloat(Integer) _index) (Math|Conversions|ToFloat(Integer) _outeriterations))))) (/ (Math|Conversions|ToFloat(Integer) _index_2) (Math|Conversions|ToFloat(Integer) Iterations))) (LocalVariables|GetEstimatedTime)))) (Math|Float|Absolute(Float) (LocalVariables|GetBestTimeDiff)))
        (LocalVariables|SetBestTimeDiff (- (CallFunction|TravelTime BulletVelocity Origin (+ Target (* Velocity (* (Math|Float|Lerp (- 1.0 (* (Math|Float|MakeLiteralFloat 1.5) (- 1.0 (/ (Math|Conversions|ToFloat(Integer) _index) (Math|Conversions|ToFloat(Integer) _outeriterations))))) (+ 1.0 (* (Math|Float|MakeLiteralFloat 1.5) (- 1.0 (/ (Math|Conversions|ToFloat(Integer) _index) (Math|Conversions|ToFloat(Integer) _outeriterations))))) (/ (Math|Conversions|ToFloat(Integer) _index_2) (Math|Conversions|ToFloat(Integer) Iterations))) (LocalVariables|GetEstimatedTime))))) (* (Math|Float|Lerp (- 1.0 (* (Math|Float|MakeLiteralFloat 1.5) (- 1.0 (/ (Math|Conversions|ToFloat(Integer) _index) (Math|Conversions|ToFloat(Integer) _outeriterations))))) (+ 1.0 (* (Math|Float|MakeLiteralFloat 1.5) (- 1.0 (/ (Math|Conversions|ToFloat(Integer) _index) (Math|Conversions|ToFloat(Integer) _outeriterations))))) (/ (Math|Conversions|ToFloat(Integer) _index_2) (Math|Conversions|ToFloat(Integer) Iterations))) (LocalVariables|GetEstimatedTime))))
        (LocalVariables|SetBestLocation (+ Target (* Velocity (* (Math|Float|Lerp (- 1.0 (* (Math|Float|MakeLiteralFloat 1.5) (- 1.0 (/ (Math|Conversions|ToFloat(Integer) _index) (Math|Conversions|ToFloat(Integer) _outeriterations))))) (+ 1.0 (* (Math|Float|MakeLiteralFloat 1.5) (- 1.0 (/ (Math|Conversions|ToFloat(Integer) _index) (Math|Conversions|ToFloat(Integer) _outeriterations))))) (/ (Math|Conversions|ToFloat(Integer) _index_2) (Math|Conversions|ToFloat(Integer) Iterations))) (LocalVariables|GetEstimatedTime)))))))
    (LocalVariables|SetEstimatedTime (CallFunction|TravelTime BulletVelocity Origin (LocalVariables|GetBestLocation))))
  (return (LocalVariables|GetBestLocation)))

(fn CalculateShot
  (params (Bullet%20Start :type Vector) (Bullet%20Speed :type Float%20%28single-precision%29) (Target%20Pos :type Vector) (Target%20Vel :type Vector))
  (LocalVariables|SetToTarget (- Target%20Pos Bullet%20Start))
  (LocalVariables|Seta (- (Math|Vector|VectorLengthSquared Target%20Vel) (Math|Float|Square Bullet%20Speed)))
  (LocalVariables|Setb (* (Math|Vector|DotProduct Target%20Vel (LocalVariables|GetToTarget)) 2.0))
  (LocalVariables|Setc (Math|Vector|VectorLengthSquared (LocalVariables|GetToTarget)))
  (LocalVariables|Setp (/ (* (LocalVariables|Getb) -1.0) (* (LocalVariables|Geta) 2.0)))
  (LocalVariables|Setq (/ (Math|Float|Sqrt (- (Math|Float|Square (LocalVariables|Getb)) (* 4.0 (LocalVariables|Geta) (LocalVariables|Getc)))) (* (LocalVariables|Geta) 2.0)))
  (LocalVariables|Sett1 (- (LocalVariables|Getp) (LocalVariables|Getq)))
  (LocalVariables|Sett2 (+ (LocalVariables|Getp) (LocalVariables|Getq)))
  (if (and (> (LocalVariables|Gett1) (LocalVariables|Gett2)) (> (LocalVariables|Gett2) 0.0))
    (return (LocalVariables|Gett2) (+ Target%20Pos (* Target%20Vel (LocalVariables|Gett2))))
    (else
      (return (LocalVariables|Gett1) (+ Target%20Pos (* Target%20Vel (LocalVariables|Gett1)))))))

(fn TrackObjectVelocity
  (params (NewPos :type Vector) (PrevPos :type Vector) (dt :type Float%20%28single-precision%29))
  (return (/ (- NewPos PrevPos) dt)))