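; Spline-driven road generator that lays a road along a spline and populates it with target dummies at play start.
; The construction script optionally snaps spline points to the ground with vertical line traces, then adds a spline mesh per segment.
; BeginPlay spawns a BP_TargetDummy at each spline point, randomly offset left or right by ObjectSpacing.
; Disconnected construction nodes hold unused ground-traced, alternating-side static mesh placement.
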(event EventBeginPlay
  (bind _spline (Variables|Default|GetSpline))
  (for _index (range 0 (- (Spline|GetNumberOfSplinePoints (Variables|Default|GetSpline)) 1))
    (Game|SpawnActorfromClass "/Game/Blueprints/BP_TargetDummy.BP_TargetDummy_C" (Math|Transform|MakeTransform (+ (Utilities|Select :Index (Math|Random|RandomIntegerinRange 0 1) :Option%200 (+ (Spline|GetLocationatSplinePoint _spline _index "World") (* (Class|SplineComponent|GetRightVectoratSplinePoint _spline _index "World") (Variables|Default|GetObjectSpacing))) :Option%201 (+ (Math|Vector|NegateVector (* (Class|SplineComponent|GetRightVectoratSplinePoint _spline _index "World") (Variables|Default|GetObjectSpacing))) (Spline|GetLocationatSplinePoint _spline _index "World"))) "0, 0,50.000000") (Spline|GetRotationatSplinePoint (Variables|Default|GetSpline) _index "World") "1,1,1") "Undefined" 0 0)))

(fn ConstructionScript
  (CallFunction|SetupRoad))

(fn AlignSplinetoGround
  (bind _spline (Variables|Default|GetSpline))
  (for _index (range 0 (- (Spline|GetNumberOfSplinePoints _spline) 1))
    (bind _outhit (Collision|LineTraceByChannel (+ (Spline|GetLocationatSplinePoint _spline _index "World") "0, 0,1000.000000") (- (Spline|GetLocationatSplinePoint _spline _index "World") "0, 0,1000.000000") "TraceTypeQuery1" false 0 "ForOneFrame"))
    (Spline|SetLocationatSplinePoint (Variables|Default|GetSpline) _index (+ (.impactpoint _outhit) (* (Transformation|GetActorUpVector) 5.0)) "World" true)))

(fn SetupRoad
  (bind _spline (Variables|Default|GetSpline))
  (if (Variables|Default|GetbGroundSpline)
    (CallFunction|AlignSplinetoGround))
  (for _index (range 0 (- (Spline|GetNumberOfSplinePoints (Variables|Default|GetSpline)) 2))
    (LocalVariables|SetCurrentIndex _index)
    (bind _returnvalue (AddComponent|AddSplineMeshComponent false))
    (SplineMesh|SetStartandEnd _returnvalue (Spline|GetLocationatSplinePoint _spline (LocalVariables|GetCurrentIndex) "Local") (Spline|GetTangentatSplinePoint _spline (LocalVariables|GetCurrentIndex) "Local") (Spline|GetLocationatSplinePoint _spline (+ (LocalVariables|GetCurrentIndex) 1) "Local") (Spline|GetTangentatSplinePoint _spline (+ (LocalVariables|GetCurrentIndex) 1) "Local") true :!class /Script/Engine.SplineMeshComponent)))