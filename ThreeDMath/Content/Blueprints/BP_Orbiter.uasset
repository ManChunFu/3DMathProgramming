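; BP_Orbiter moves a sphere along three nested orbits around the actor, tracing them with debug points and circles.
; OrbitSolver derives position and angle from game time, and each orbit adds to its parent's position, with the first stretched on Y and the second tilted.
; Tick places the sphere on the innermost orbit and drives a top-down spring arm.
; Q cycles the camera between an overview and each orbit, matching position, yaw and arm length.
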(event EventTick
  (params (DeltaSeconds :type Float%20%28single-precision%29))
  (bind (_returnvalue _radiusout _degrees) (CallFunction|OrbitSolver 5e+01 0.0 6.8e+02))
  (bind (_returnvalue_2 _radiusout_2 _degrees_2) (CallFunction|OrbitSolver 1.5e+02 11.0 3.6e+02))
  (bind _radius (Variables|Default|GetRadius))
  (bind _offset (Variables|Default|GetOffset))
  (bind _rate (Variables|Default|GetRate))
  (bind (_returnvalue_3 _radiusout_3 _degrees_3) (CallFunction|OrbitSolver _radius _offset _rate))
  (bind _returnvalue_4 (Math|Vector|RotateVector _returnvalue_2 "0, 0,30.000000"))
  (bind _returnvalue_5 (* _returnvalue_3 "1.000000,2.000000,1.000000"))
  (bind _return_value (CallFunction|DrawOrbits _returnvalue_5 "(R=0.250612,G=1.000000,B=0.067781,A=1.000000)" _radiusout_3 true "0, 0, 0"))
  (bind _returnvalue_6 (+ _return_value _returnvalue_4))
  (bind _return_value_2 (CallFunction|DrawOrbits _returnvalue_6 "(R=0.947917,G=0.051326,B=0.596622,A=1.000000)" _radiusout_2 true _return_value))
  (bind _returnvalue_7 (+ _return_value_2 _returnvalue))
  (bind _return_value_3 (CallFunction|DrawOrbits _returnvalue_7 "(R=0.008445,G=0.036314,B=1.000000,A=1.000000)" _radiusout true _return_value_2))
  (Transformation|SetRelativeLocationAndRotation (Variables|Default|GetSpringArm) (Utilities|Select :Index (Variables|Default|GetCameraInt) :Option%200 "0, 0, 0" :Option%201 _return_value :Option%202 _return_value_2 :Option%203 _return_value_3) (Math|Rotator|MakeRotator 0.0 -9e+01 (Utilities|Select :Index (Variables|Default|GetCameraInt) :Option%200 0.0 :Option%201 _degrees_3 :Option%202 _degrees_2 :Option%203 _degrees)) false false)
  (Variables|/Script/Engine.SpringArmComponent|SetTargetArmLength (Variables|Default|GetSpringArm) (Utilities|Select :Index (Variables|Default|GetCameraInt) :Option%200 2e+03 :Option%201 (* _radiusout_3 2.0) :Option%202 (* _radiusout_2 2.0) :Option%203 (* _radiusout 2.0)))
  (Transformation|SetRelativeLocation (Variables|Default|GetSphere) _return_value_3 false false))

(event Input|KeyboardEvents|Q
  (params (Key :type Key%20Structure :default "None"))
  (:Pressed
    (bind _result (Math|Integer|IncrementInt (Variables|Default|GetCameraInt))
      (:%20%20
        (Variables|Default|SetCameraInt (Math|Integer|%(Integer) _result 4))))))

(fn ConstructionScript
  (Transformation|SetRelativeLocation (Variables|Default|GetSphere) (Math|Vector|RotateVector (Math|Vector|MakeVector (Variables|Default|GetRadius) 0.0 0.0) (Math|Rotator|MakeRotator 0.0 0.0 (Math|Float|Absolute(Float) (Math|Float|%(Float) (Variables|Default|GetOffset) 3.6e+02)))) false false))

(fn OrbitSolver
  (params (Radius :type Float%20%28single-precision%29) (Offset :type Float%20%28single-precision%29) (Rate :type Float%20%28single-precision%29))
  (bind _returnvalue (Utilities|Time|GetGameTimeinSeconds))
  (bind _returnvalue_2 (* Rate _returnvalue))
  (bind _returnvalue_3 (+ Offset _returnvalue_2))
  (bind _returnvalue_4 (Math|Float|%(Float) _returnvalue_3 3.6e+02))
  (bind _returnvalue_5 (Math|Float|Absolute(Float) _returnvalue_4))
  (return (Math|Vector|RotateVector (Math|Vector|MakeVector Radius 0.0 0.0) (Math|Rotator|MakeRotator 0.0 0.0 _returnvalue_5)) Radius _returnvalue_5))

(fn DrawOrbits
  (params (Orbit%20Pos :type Vector) (PointColor :type Linear%20Color%20Structure) (Radius :type Float%20%28single-precision%29) (Draw%20Circle :type Boolean) (Parent%20Orbit%20Pos :type Vector))
  (Rendering|Debug|DrawDebugPoint (+ Orbit%20Pos (Transformation|GetActorLocation)) 3.0 PointColor 15.0)
  (if Draw%20Circle
    (Rendering|Debug|DrawDebugCircle (+ Parent%20Orbit%20Pos (Transformation|GetActorLocation)) Radius 64 PointColor 0.0 1e+01 "1.000000,0.000000,0.000000" "0.000000,1.000000,0.000000"))
  (return Orbit%20Pos))