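; BP_TestTurret is a turret that aims and lobs BP_TestTurretBall projectiles at a moving target within range.
; A looping timer with randomized start fires it, while Tick yaws the actor, pitches the barrel and draws the predicted arc.
; Ballistic math derives launch speed from range and muzzle height, then solves a high or low trajectory.
; Aim leads the target by its velocity times a flight time estimated from current barrel pitch.
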(event Custom|Fire
  (if (CallFunction|IsTargetWithinRange)
    ;[1 1 1] Spawn BP_CannonBall
    (bind _returnvalue (Game|SpawnActorfromClass "/Game/Blueprints/BP_TestTurretBall.BP_TestTurretBall_C" (Math|Transform|MakeTransform (Transformation|GetWorldLocation (Variables|Default|GetMuzzle)) (Transformation|GetWorldRotation (Variables|Default|GetHead)) "1,1,1") "AlwaysSpawn" self 0))
    (Variables|/Game/Blueprints/BP_TestTurretBall.BP_TestTurretBall_C|SetLaunchVelocity _returnvalue (CallFunction|GetLaunchVelocity))))

(event Custom|CallFire
  (CallFunction|Fire))

(event EventBeginPlay
  (Utilities|Time|SetTimerbyEvent (delegate Custom|CallFire) (Variables|Default|GetFireRate) true 0.0 1.0))

(event EventTick
  (params (DeltaSeconds :type Float%20%28single-precision%29))
  (Transformation|SetRelativeRotation (Variables|Default|GetBarrel) (Math|Rotator|MakeRotator 0.0 (.pitch (Math|Rotator|FindLookatRotation (Transformation|GetActorLocation) (CallFunction|GetLaunchVelocity))) 0.0) false false)
  (Transformation|SetActorRotation (Math|Rotator|MakeRotator 0.0 0.0 (.yaw (Math|Rotator|FindLookatRotation (Transformation|GetActorLocation) (CallFunction|GetPredictPosition)))))
  (if (CallFunction|IsTargetWithinRange)
    (Class|GameplayStatics|BlueprintPredictProjectilePathbyTraceChannel (Transformation|GetWorldLocation (Variables|Default|GetMuzzle)) (CallFunction|GetLaunchVelocity) false 0.0 "ECC_WorldDynamic" false 0 "ForOneFrame" 2.0 1e+01 5.0)))

(fn ConstructionScript)

(fn GetLaunchSpeed
  (bind _range (Variables|Default|GetRange))
  (bind _muzzle (Variables|Default|GetMuzzle))
  (bind _returnvalue (Transformation|GetWorldLocation _muzzle))
  (bind _output_get (Variables|Default|SetLaunchSpeed (Math|Float|Sqrt (* (Variables|Default|GetGravity) (Math|Float|Sqrt (+ (* _range _range) (* (.z _returnvalue) (.z _returnvalue))))))))
  (return _output_get))

(fn IsTargetWithinRange
  (Variables|Default|GetTarget
    (:then
      (return (<= (Math|Vector|Distance(Vector) (Transformation|GetActorLocation) (Transformation|GetActorLocation (Variables|Default|GetTarget))) (Variables|Default|GetRange))))
    (:else
      (return false))))

(fn GetLaunchVelocity
  (LocalVariables|SetDirToTarget (Math|Vector|Normalize (- (CallFunction|GetPredictPosition) (Transformation|GetActorLocation))))
  (bind _output_get (LocalVariables|Sets (CallFunction|GetLaunchSpeed)))
  (LocalVariables|Sets2 (* _output_get _output_get))
  (LocalVariables|Setx (Math|Vector|Distance(Vector) (Transformation|GetActorLocation) (CallFunction|GetPredictPosition)))
  (LocalVariables|Sety (.z (Transformation|GetWorldLocation (Variables|Default|GetMuzzle))))
  (LocalVariables|SetRootContent (- (* (LocalVariables|Gets2) (LocalVariables|Gets2)) (* (Variables|Default|GetGravity) (+ (* (Variables|Default|GetGravity) (LocalVariables|Getx) (LocalVariables|Getx)) (* 2.0 (LocalVariables|Gety) (LocalVariables|Gets2))))))
  (if (Variables|Default|GetbHighTrajectory)
    (bind _output_get_2 (LocalVariables|SetTanTheta (/ (+ (LocalVariables|Gets2) (Math|Float|Sqrt (LocalVariables|GetRootContent))) (* (Variables|Default|GetGravity) (LocalVariables|Getx)))))
    (else
      (LocalVariables|SetTanTheta (/ (- (LocalVariables|Gets2) (Math|Float|Sqrt (LocalVariables|GetRootContent))) (* (Variables|Default|GetGravity) (LocalVariables|Getx))))))
  (bind _output_get_3 (LocalVariables|SetCosTheta (Math|Trig|Cos(Radians) (Math|Trig|Atan(Degrees) _output_get_2))))
  (LocalVariables|SetSinTheta (* _output_get_3 (LocalVariables|GetTanTheta)))
  (return (Math|Vector|MakeVector (* (LocalVariables|Gets) (LocalVariables|GetCosTheta) (.x (LocalVariables|GetDirToTarget))) (* (LocalVariables|Gets) (LocalVariables|GetCosTheta) (.y (LocalVariables|GetDirToTarget))) (* (LocalVariables|Gets) (LocalVariables|GetSinTheta)))))

(fn GetFlightTime
  (bind _returnvalue (Transformation|GetActorLocation))
  (return (/ (* 2.0 (CallFunction|GetLaunchSpeed) (Math|Trig|Sin(Degrees) (.pitch (Math|Rotator|FindLookatRotation _returnvalue (+ _returnvalue (Math|Vector|GetForwardVector (Variables|Default|GetBarrel))))))) (Variables|Default|GetGravity))))

(fn GetPredictPosition
  (bind _target (Variables|Default|GetTarget))
  (return (+ (Transformation|GetActorLocation _target) (* (Transformation|GetVelocity _target) (CallFunction|GetFlightTime)))))