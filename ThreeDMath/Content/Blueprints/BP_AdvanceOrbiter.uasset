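; Solar system actor that builds a star and orbiting bodies from the SolarSystemDeets data table and animates them over game time.
; The construction script spawns a mesh per table row, using OrbitSolver for its position, scale and color.
; Tick re-runs OrbitSolver with debug enabled to move each body.
; Q cycles a four-state CameraInt, which nothing in this graph reads.
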(event EventTick
  (params (DeltaSeconds :type Float%20%28single-precision%29))
  (bind _celestialbodies (Variables|Default|GetCelestialBodies))
  (for (_array_element _array_index) (Variables|Default|GetBodyArray)
    (Transformation|SetRelativeLocation _array_element (.Solution (CallFunction|OrbitSolver self (Utilities|Array|Get(acopy) _celestialbodies _array_index) true _celestialbodies (Utilities|Time|GetGameTimeinSeconds))) false false)))

(event Input|KeyboardEvents|Q
  (params (Key :type Key%20Structure))
  (:Pressed
    (bind _result (Math|Integer|IncrementInt (Variables|Default|GetCameraInt))
      (:%20%20
        (Variables|Default|SetCameraInt (Math|Integer|%(Integer) _result 4))))))

(fn ConstructionScript
  (bind _solarsystemdeets (Variables|Default|GetSolarSystemDeets))
  (Utilities|Array|Clear (Variables|Default|GetBodyArray))
  (Utilities|Array|Clear (Variables|Default|GetCelestialBodies))
  (bind _outrownames (DataTable|GetDataTableRowNames _solarsystemdeets))
  (for _array_element _outrownames
    (bind _returnvalue (Utilities|GetDataTableRow _solarsystemdeets _array_element)
      (:then
        (Utilities|Array|Add (Variables|Default|GetCelestialBodies) _returnvalue))))
  (AddComponent|AddStaticMeshComponent false (Math|Transform|MakeTransform "0, 0, 0" "0, 0, 0" (Math|Conversions|ToVector(Float) (Variables|Default|GetStarRadius))))
  (for _array_element_2 (Variables|Default|GetCelestialBodies)
    (bind _returnvalue_2 (AddComponent|AddStaticMeshComponent false (Math|Transform|MakeTransform (.Solution (CallFunction|OrbitSolver self _array_element_2 false (Variables|Default|GetCelestialBodies) 0.0)) "0, 0, 0" (Math|Conversions|ToVector(Float) (.PlanetScale (CallFunction|OrbitSolver self _array_element_2 false (Variables|Default|GetCelestialBodies) 0.0))))))
    (Rendering|Material|SetVectorParameterValueonMaterials _returnvalue_2 "Color" (Math|Conversions|ToVector(LinearColor) (.Color (CallFunction|OrbitSolver self _array_element_2 false (Variables|Default|GetCelestialBodies) 0.0))))
    (Utilities|Array|Add (Variables|Default|GetBodyArray) _returnvalue_2)))