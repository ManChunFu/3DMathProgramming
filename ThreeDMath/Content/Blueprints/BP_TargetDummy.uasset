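; BP_TargetDummy is a target dummy actor that reports the damage it takes and removes itself when killed.
; It reacts to events from its BP_HealthComponent.
; OnDamageTaken prints the actor's name and current health, while OnDeath prints a death message and destroys the actor.
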(event OnDamageTaken(BP_HealthComponent)
  (params (CurrentHealth :type Float%20%28single-precision%29))
  (Development|PrintString (Utilities|String|Append (Utilities|GetDisplayName self) " has taken Damage! Current Health: " (Utilities|String|ToString(Float) CurrentHealth))))

(event OnDeath(BP_HealthComponent)
  (Development|PrintString (Utilities|String|Append (Utilities|GetDisplayName self) " is dead."))
  (Actor|DestroyActor))

(fn ConstructionScript)