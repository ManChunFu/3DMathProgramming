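; Health component that tracks CurrentHealth for its owning actor and reports damage and death.
; On BeginPlay it binds to the owner's OnTakeAnyDamage and subtracts any positive damage from CurrentHealth, without clamping.
; Each such hit broadcasts OnDamageTaken with the new health, then OnDeath if IsDead finds health at or below zero.
; OnDeath has no one-shot guard, so further hits on a dead owner broadcast it again.
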(event Custom|OnTakeAnyDamage_Event_0
  (params (DamagedActor :type Actor%20Object%20Reference) (Damage :type Float%20%28single-precision%29) (DamageType :type Damage%20Type%20Object%20Reference) (InstigatedBy :type Controller%20Object%20Reference) (DamageCauser :type Actor%20Object%20Reference))
  (if (> Damage 0.0)
    (bind _output_get (Variables|Default|SetCurrentHealth (- (Variables|Default|GetCurrentHealth) Damage)))
    (Default|CallOnDamageTaken _output_get)
    (if (CallFunction|IsDead)
      (Default|CallOnDeath))))

(event EventBeginPlay
  (EventDispatchers|AssignOnTakeAnyDamage (Components|GetOwner) (delegate Custom|OnTakeAnyDamage_Event_0)))

(fn IsDead
  (return (>= 0.0 (Variables|Default|GetCurrentHealth))))