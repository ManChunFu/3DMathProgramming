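; BP_Cannon is a cannon actor that fires a cannon ball when its OnFire event runs.
; It spawns the configured ball class at the muzzle with the head mesh's relative rotation, then passes launch speed, angle and gravity to BP_CannonBall's Setup.
; It also draws a brief debug predicted path from the barrel's location and forward vector, scaling launch speed by 100.
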(event EventOnFire
  (bind _self self)
  (bind _barrelmesh (Variables|Default|GetBarrelMesh))
  ;[1 1 1] Spawn BP_CannonBall
  (bind _returnvalue (Game|SpawnActorfromClass (Variables|Default|GetCannonBallToSpawn) (Math|Transform|MakeTransform (Transformation|GetWorldLocation (Variables|Default|GetCannonMuzzle)) (Variables|/Script/Engine.SceneComponent|GetRelativeRotation (Variables|Default|GetCannonHeadMesh)) "1,1,1") "AlwaysSpawn" _self _self))
  ;[1 1 1] Set up the cannon ball's variables
  (bind _asbp_cannon_ball (Utilities|Casting|CastToBP_CannonBall _returnvalue))
  (Default|Setup _asbp_cannon_ball (Variables|Default|GetLaunchSpeed) (Variables|Default|GetLaunchAngleInRad) (Variables|Default|GetGravity))
  ;[1 1 1] Debug trajectory path
  (Class|GameplayStatics|BlueprintPredictProjectilePathbyTraceChannel (Transformation|GetWorldLocation _barrelmesh) (* (Math|Vector|GetForwardVector _barrelmesh) (* (Variables|Default|GetLaunchSpeed) 1e+02)) false 0.0 "ECC_WorldDynamic" false 0 "ForDuration" 2.0))

(fn ConstructionScript)