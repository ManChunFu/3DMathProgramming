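; Blueprint function library that computes a celestial body's position, color and scale from its orbit data and a time value.
; OrbitSolver recursively adds the parent body's position, so nested orbits such as moons follow their parents.
; It rotates a radius vector at a speed inversely proportional to radius, with optional direction reversal, then applies shape, skew and ecliptic tilt.
; In debug mode, DrawOrbit plots colored points relative to the context actor.
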(fn OrbitSolver
  (params (Context :type Actor%20Object%20Reference) (Orbit :type BP%20Orbit%20Params%20Structure) (Debug :type Boolean) (Bodies :type Array%20of%20BP%20Orbit%20Params%20Structures) (Time :type Float%20%28single-precision%29))
  (bind _returnvalue (/ (.orbitalradius Orbit) 1.5e+04))
  (bind _returnvalue_2 (/ 3.65 _returnvalue))
  (bind _returnvalue_3 (* _returnvalue_2 Time))
  (bind _returnvalue_4 (+ (.timeoffset Orbit) _returnvalue_3))
  (if (> (.parentalbody Orbit) -1)
    (LocalVariables|SetParentalOrbit (.Solution (CallFunction|OrbitSolver Context (Utilities|Array|Get(acopy) Bodies (.parentalbody Orbit)) false Bodies Time Context))))
  (if Debug
    (CallFunction|DrawOrbit Context (+ (LocalVariables|GetParentalOrbit) (Math|Vector|RotateVector (+ (* (Math|Vector|RotateVector (Math|Vector|MakeVector (.orbitalradius Orbit) 0.0 0.0) (Math|Rotator|MakeRotator 0.0 0.0 (Math|Float|%(Float) (Math|Float|SelectFloat (* _returnvalue_4 -1.0) _returnvalue_4 (.antipodal Orbit)) 3.6e+02))) (Math|Vector|MakeVector 1.0 (+ (.orbitalshape Orbit) 1.0) 1.0)) (Math|Vector|MakeVector (* (.orbitalradius Orbit) (.orbitalskew Orbit)) 0.0 0.0)) (.eclipticoffset Orbit))) (.planetcolor Orbit) Context))
  (return (+ (LocalVariables|GetParentalOrbit) (Math|Vector|RotateVector (+ (* (Math|Vector|RotateVector (Math|Vector|MakeVector (.orbitalradius Orbit) 0.0 0.0) (Math|Rotator|MakeRotator 0.0 0.0 (Math|Float|%(Float) (Math|Float|SelectFloat (* _returnvalue_4 -1.0) _returnvalue_4 (.antipodal Orbit)) 3.6e+02))) (Math|Vector|MakeVector 1.0 (+ (.orbitalshape Orbit) 1.0) 1.0)) (Math|Vector|MakeVector (* (.orbitalradius Orbit) (.orbitalskew Orbit)) 0.0 0.0)) (.eclipticoffset Orbit))) (.planetcolor Orbit) (.planetscale Orbit)))

(fn DrawOrbit
  (params (Context :type Actor%20Object%20Reference) (OrbitPos :type Vector) (PointColor :type Linear%20Color%20Structure))
  (Rendering|Debug|DrawDebugPoint Context (+ OrbitPos (Transformation|GetActorLocation Context)) 3.0 PointColor 15.0))