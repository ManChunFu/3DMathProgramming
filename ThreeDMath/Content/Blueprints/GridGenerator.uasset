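; GridGenerator is a Blueprint actor that lays out a two-dimensional grid of static mesh components.
; Its construction script runs nested loops over GridX and GridY, adding one component per cell at index times Spacing on X and Y with a uniform Scale.
; The event graph holds only disabled default events, so all of the work happens at construction.
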(event EventBeginPlay)

(event Collision|EventActorBeginOverlap
  (params (OtherActor :type Actor%20Object%20Reference)))

(event EventTick
  (params (DeltaSeconds :type Float%20%28single-precision%29)))

(fn ConstructionScript
  (for _index (range 0 (- (Variables|Default|GetGridX) 1))
    (for _index_2 (range 0 (- (Variables|Default|GetGridY) 1))
      (AddComponent|AddStaticMeshComponent false (Math|Transform|MakeTransform (Math|Vector|MakeVector (* _index (Variables|Default|GetSpacing)) (* _index_2 (Variables|Default|GetSpacing)) 0.0) "0, 0, 0" (Math|Conversions|ToVector(Float) (Variables|Default|GetScale)))))))