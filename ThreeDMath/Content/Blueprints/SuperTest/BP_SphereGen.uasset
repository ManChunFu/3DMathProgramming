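; BP_SphereGen is an actor Blueprint that attempts to generate a procedural sphere mesh in its construction script.
; Nested stack and sector loops compute vertices from Radius and append normals scaled by its inverse, then create a mesh section.
; The script never fills Triangles or UVs.
; Angle steps are in radians but feed degree-based trig, and the stack angle subtracts the index before multiplying by the step.
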(event EventBeginPlay)

(event Collision|EventActorBeginOverlap
  (params (OtherActor :type Actor%20Object%20Reference)))

(event EventTick
  (params (DeltaSeconds :type Float%20%28single-precision%29)))

(fn ConstructionScript
  (Variables|Default|SetSectorStep (/ (* 2 (Math|Trig|GetPI)) (Variables|Default|GetSectorCount)))
  (Variables|Default|SetStackStep (/ (Math|Trig|GetPI) (Variables|Default|GetStackCount)))
  (for _index (range 0 (Math|Float|Truncate (- (Variables|Default|GetStackCount) 1.0)))
    (Variables|Default|SetStackAngle (* (- (/ (Math|Trig|GetPI) 2.0) (Math|Conversions|ToFloat(Integer) _index)) (Variables|Default|GetStackStep)))
    (Variables|Default|SetXY (* (Variables|Default|GetRadius) (Math|Trig|Cos(Degrees) (Variables|Default|GetStackAngle))))
    (Variables|Default|SetZ (* (Variables|Default|GetRadius) (Math|Trig|Sin(Degrees) (Variables|Default|GetStackAngle))))
    (for _index_2 (range 0 (Math|Float|Truncate (- (Variables|Default|GetSectorCount) 1.0)))
      (Variables|Default|SetSectorAngle (* _index_2 (Variables|Default|GetSectorStep)))
      (Variables|Default|SetX (* (Variables|Default|GetXY) (Math|Trig|Cos(Degrees) (Variables|Default|GetSectorAngle))))
      (Variables|Default|SetY (* (Variables|Default|GetXY) (Math|Trig|Sin(Degrees) (Variables|Default|GetSectorAngle))))
      (bind _returnvalue (Utilities|Array|Add (Variables|Default|GetVertices) (Math|Vector|MakeVector (Variables|Default|GetX) (Variables|Default|GetY) (Variables|Default|GetZ))))
      (Utilities|Array|Add (Variables|Default|GetNormals) (* (Utilities|Array|Get(acopy) (Variables|Default|GetVertices) _returnvalue) (/ 1.0 (Variables|Default|GetRadius))))))
  (Class|ProceduralMeshComponent|CreateMeshSectionLinearColor (Variables|Default|GetProceduralMesh) 0 (Variables|Default|GetVertices) (Variables|Default|GetTriangles) (Variables|Default|GetNormals) (Variables|Default|GetUV0) 0 0 0 (Variables|Default|GetVertex%20Colors) (Variables|Default|GetTangents) false))