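; BP_GroundTile is a ground tile actor that builds its own box-shaped mesh.
; The construction script generates box geometry from GroundSize and writes it to the ProceduralMesh component with collision enabled.
; An unconnected node chain that would add a BlockAll box collider of the same extent never runs, and the event graph holds only empty events.
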(event EventBeginPlay)

(event Collision|EventActorBeginOverlap
  (params (OtherActor :type Actor%20Object%20Reference)))

(event EventTick
  (params (DeltaSeconds :type Float%20%28single-precision%29)))

(fn ConstructionScript
  (bind (_vertices _triangles _normals _uvs _tangents) (Class|KismetProceduralMeshLibrary|GenerateBoxMesh (Variables|Default|GetGroundSize)))
  (Class|ProceduralMeshComponent|CreateMeshSectionLinearColor (Variables|Default|GetProceduralMesh) 0 _vertices _triangles _normals _uvs 0 0 0 0 _tangents true))