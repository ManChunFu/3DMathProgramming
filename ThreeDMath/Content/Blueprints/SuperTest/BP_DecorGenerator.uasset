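; Decor actor that builds a procedural cone, cylinder or sphere mesh in the Construction Script, selected by Shape.
; Each Draw function sweeps rings of vertices around the up vector, derives grid triangles, normals and tangents, then feeds one mesh section.
; The cone scales radius by height minus a cut-off.
; DrawSphere currently duplicates the cylinder math, and the triangle and quad functions are not called.
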(event EventBeginPlay)

(event Collision|EventActorBeginOverlap
  (params (OtherActor :type Actor%20Object%20Reference)))

(event EventTick
  (params (DeltaSeconds :type Float%20%28single-precision%29)))

(fn ConstructionScript
  (CallFunction|ClearMeshData)
  (switch Utilities|FlowControl|Switch|SwitchonEShappe (Variables|Default|GetShape)
    (:NewEnumerator1
      (CallFunction|DrawCone))
    (:NewEnumerator0
      (CallFunction|DrawCylinder))
    (:NewEnumerator3
      (CallFunction|DrawSphere)))
  (Class|ProceduralMeshComponent|CreateMeshSectionLinearColor (Variables|Default|GetProceduralMesh) 0 (Variables|Default|GetVertices) (Variables|Default|GetTriangle) (Variables|Default|GetNormals) (Variables|Default|GetUV) 0 0 0 (Variables|Default|GetVertexColors) (Variables|Default|GetTangents) false))

(fn DrawTriangle
  (Variables|Default|SetVertices (Utilities|Array|MakeArray "0, 0, 0" "0, 0,200.000000" "200.000000, 0, 0"))
  (Variables|Default|SetTriangle (Utilities|Array|MakeArray 2 1 0)))

(fn DrawQuad
  (for _index (range 0 (Variables|Default|GetXLength))
    (Variables|Default|SetX _index)
    (for _index_2 (range 0 (Variables|Default|GetYLength))
      (Variables|Default|SetY _index_2)
      (Utilities|FlowControl|Sequence
        (:then_0
          (Utilities|Array|Add (Variables|Default|GetVertices) (Math|Vector|MakeVector (* (Variables|Default|GetX) 5e+01) 0.0 (* (Variables|Default|GetY) 5e+01))))
        (:then_1
          (Utilities|Array|Add (Variables|Default|GetUV) (Math|Vector2D|MakeVector2D (/ (Math|Conversions|ToFloat(Integer) (Variables|Default|GetX)) (Math|Conversions|ToFloat(Integer) (Variables|Default|GetXLength))) (/ (Math|Conversions|ToFloat(Integer) (Variables|Default|GetY)) (Math|Conversions|ToFloat(Integer) (Variables|Default|GetYLength)))))))))
  (Utilities|FlowControl|Sequence
    (:then_0
      (bind _triangles (Class|KismetProceduralMeshLibrary|CreateGridMeshTriangles (+ (Variables|Default|GetXLength) 1) (+ (Variables|Default|GetYLength) 1) true))
      (Variables|Default|SetTriangle _triangles))
    (:then_1
      (bind (_normals _tangents) (Class|KismetProceduralMeshLibrary|CalculateTangentsforMesh (Variables|Default|GetVertices) (Variables|Default|GetTriangle) (Variables|Default|GetUV)))
      (Variables|Default|SetNormals _normals)
      (Variables|Default|SetTangents _tangents))))

(fn DrawCylinder
  (for _index (range 0 (Variables|Default|GetZLength))
    (Variables|Default|SetZ _index)
    (for _index_2 (range 0 (Variables|Default|GetXLength))
      (Variables|Default|SetX _index_2)
      (Utilities|FlowControl|Sequence
        (:then_0
          (Utilities|Array|Add (Variables|Default|GetVertices) (+ (* (Math|Vector|RotateVectorAroundAxis (Transformation|GetActorForwardVector) (* (/ (Math|Conversions|ToFloat(Integer) (Variables|Default|GetX)) (Math|Conversions|ToFloat(Integer) (Variables|Default|GetXLength))) 3.6e+02) (Transformation|GetActorUpVector)) (Variables|Cone|GetConeWidth)) (Math|Vector|MakeVector (Variables|Cone|GetConeXOffset) (Variables|Cone|GetConeYOffset) (* (Variables|Default|GetZ) (Variables|Cone|GetConeZOffset))))))
        (:then_1
          (Utilities|Array|Add (Variables|Default|GetUV) (Math|Vector2D|MakeVector2D (/ (Math|Conversions|ToFloat(Integer) (Variables|Default|GetZ)) (Math|Conversions|ToFloat(Integer) (Variables|Default|GetZLength))) (/ (Math|Conversions|ToFloat(Integer) (Variables|Default|GetX)) (Math|Conversions|ToFloat(Integer) (Variables|Default|GetXLength)))))))))
  (Utilities|FlowControl|Sequence
    (:then_0
      (bind _triangles (Class|KismetProceduralMeshLibrary|CreateGridMeshTriangles (+ (Variables|Default|GetZLength) 1) (+ (Variables|Default|GetXLength) 1) true))
      (Variables|Default|SetTriangle _triangles))
    (:then_1
      (bind (_normals _tangents) (Class|KismetProceduralMeshLibrary|CalculateTangentsforMesh (Variables|Default|GetVertices) (Variables|Default|GetTriangle) (Variables|Default|GetUV)))
      (Variables|Default|SetNormals _normals)
      (Variables|Default|SetTangents _tangents))))

(fn DrawCone
  (for _index (range 0 (Variables|Default|GetZLength))
    (Variables|Default|SetZ _index)
    (for _index_2 (range 0 (Variables|Default|GetXLength))
      (Variables|Default|SetX _index_2)
      (Utilities|FlowControl|Sequence
        (:then_0
          (Utilities|Array|Add (Variables|Default|GetVertices) (+ (* (Math|Vector|RotateVectorAroundAxis (Transformation|GetActorForwardVector) (* (/ (Math|Conversions|ToFloat(Integer) (Variables|Default|GetX)) (Math|Conversions|ToFloat(Integer) (Variables|Default|GetXLength))) 3.6e+02) (Transformation|GetActorUpVector)) (* (Variables|Cone|GetConeWidth) (- (/ (Math|Conversions|ToFloat(Integer) (Variables|Default|GetZ)) (Math|Conversions|ToFloat(Integer) (Variables|Default|GetZLength))) (Variables|Cone|GetConeCutOff)))) (Math|Vector|MakeVector 0.0 0.0 (* (Variables|Default|GetZ) (Variables|Cone|GetConeZOffset))))))
        (:then_1
          (Utilities|Array|Add (Variables|Default|GetUV) (Math|Vector2D|MakeVector2D (/ (Math|Conversions|ToFloat(Integer) (Variables|Default|GetZ)) (Math|Conversions|ToFloat(Integer) (Variables|Default|GetZLength))) (/ (Math|Conversions|ToFloat(Integer) (Variables|Default|GetX)) (Math|Conversions|ToFloat(Integer) (Variables|Default|GetXLength)))))))))
  (Utilities|FlowControl|Sequence
    (:then_0
      (bind _triangles (Class|KismetProceduralMeshLibrary|CreateGridMeshTriangles (+ (Variables|Default|GetZLength) 1) (+ (Variables|Default|GetXLength) 1) true))
      (Variables|Default|SetTriangle _triangles))
    (:then_1
      (bind (_normals _tangents) (Class|KismetProceduralMeshLibrary|CalculateTangentsforMesh (Variables|Default|GetVertices) (Variables|Default|GetTriangle) (Variables|Default|GetUV)))
      (Variables|Default|SetNormals _normals)
      (Variables|Default|SetTangents _tangents))))

(fn ClearMeshData
  (Utilities|Array|Clear (Variables|Default|GetVertices))
  (Utilities|Array|Clear (Variables|Default|GetTriangle))
  (Utilities|Array|Clear (Variables|Default|GetUV)))

(fn DrawSphere
  (for _index (range 0 (Variables|Default|GetZLength))
    (Variables|Default|SetZ _index)
    (for _index_2 (range 0 (Variables|Default|GetXLength))
      (Variables|Default|SetX _index_2)
      (Utilities|FlowControl|Sequence
        (:then_0
          (Utilities|Array|Add (Variables|Default|GetVertices) (+ (* (Math|Vector|RotateVectorAroundAxis (Transformation|GetActorForwardVector) (* (/ (Math|Conversions|ToFloat(Integer) (Variables|Default|GetX)) (Math|Conversions|ToFloat(Integer) (Variables|Default|GetXLength))) 3.6e+02) (Transformation|GetActorUpVector)) (Variables|Cone|GetConeWidth)) (Math|Vector|MakeVector (Variables|Cone|GetConeXOffset) (Variables|Cone|GetConeYOffset) (* (Variables|Default|GetZ) (Variables|Cone|GetConeZOffset))))))
        (:then_1
          (Utilities|Array|Add (Variables|Default|GetUV) (Math|Vector2D|MakeVector2D (/ (Math|Conversions|ToFloat(Integer) (Variables|Default|GetZ)) (Math|Conversions|ToFloat(Integer) (Variables|Default|GetZLength))) (/ (Math|Conversions|ToFloat(Integer) (Variables|Default|GetX)) (Math|Conversions|ToFloat(Integer) (Variables|Default|GetXLength)))))))))
  (Utilities|FlowControl|Sequence
    (:then_0
      (bind _triangles (Class|KismetProceduralMeshLibrary|CreateGridMeshTriangles (+ (Variables|Default|GetZLength) 1) (+ (Variables|Default|GetXLength) 1) true))
      (Variables|Default|SetTriangle _triangles))
    (:then_1
      (bind (_normals _tangents) (Class|KismetProceduralMeshLibrary|CalculateTangentsforMesh (Variables|Default|GetVertices) (Variables|Default|GetTriangle) (Variables|Default|GetUV)))
      (Variables|Default|SetNormals _normals)
      (Variables|Default|SetTangents _tangents))))