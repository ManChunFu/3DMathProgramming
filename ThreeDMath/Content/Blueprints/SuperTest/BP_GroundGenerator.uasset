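; Ground generator actor that builds a block of BP_GroundTile actors when play begins.
; GenerateFloor runs nested loops over the X, Z and Y lengths, spawning tiles at fixed spacing and attaching each to itself.
; The Z index runs along world Y, while the Y index stacks layers downward.
; Unconnected leftovers hold a trace-based procedural mesh slicing test and construction-time floor and box mesh generation.
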(event EventBeginPlay
  (CallFunction|GenerateFloor))

(fn ConstructionScript)

(fn GenerateFloor
  (for _index (range 0 (Variables|Default|GetZLength))
    (Variables|Default|SetZ _index)
    (for _index_2 (range 0 (Variables|Default|GetXLength))
      (Variables|Default|SetX (Math|Conversions|ToFloat(Integer) _index_2))
      (for _index_3 (range 0 (Variables|Default|GetYLength))
        (Variables|Default|SetY (Math|Conversions|ToFloat(Integer) _index_3))
        (bind _returnvalue (Game|SpawnActorfromClass "/Game/Blueprints/SuperTest/BP_GroundTile.BP_GroundTile_C" (Math|Transform|MakeTransform (+ (Transformation|GetActorLocation) (Math|Vector|MakeVector (* (Variables|Default|GetX) 4e+02) (* (Math|Conversions|ToFloat(Integer) (Variables|Default|GetZ)) 4e+02) (* (Variables|Default|GetY) -4e+02))) "0, 0, 0" "1,1,1") "AlwaysSpawn" 0 0))
        (Transformation|AttachActorToActor _returnvalue self "None" "KeepWorld" "KeepWorld" "KeepWorld" true)))))