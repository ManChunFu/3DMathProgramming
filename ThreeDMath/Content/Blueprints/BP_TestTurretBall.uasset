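; BP_TestTurretBall is a test projectile actor that flies along a ballistic arc from where it spawns.
; BeginPlay stores its location as the launch point, and Tick accumulates elapsed time.
; Each Tick sets the position analytically from launch velocity and time, subtracting a gravity drop on Z.
; The move is done without sweep, so it does not check for collisions along the path.
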(event EventTick
  (params (DeltaSeconds :type Float%20%28single-precision%29))
  (Variables|Default|SetTimePassed (+ DeltaSeconds (Variables|Default|GetTimePassed)))
  (Transformation|SetActorLocation (Math|Vector|MakeVector (.x (+ (Variables|Default|GetLaunchPoint) (* (Variables|Default|GetLaunchVelocity) (Variables|Default|GetTimePassed)))) (.y (+ (Variables|Default|GetLaunchPoint) (* (Variables|Default|GetLaunchVelocity) (Variables|Default|GetTimePassed)))) (- (.z (+ (Variables|Default|GetLaunchPoint) (* (Variables|Default|GetLaunchVelocity) (Variables|Default|GetTimePassed)))) (* 0.5 (Variables|Default|GetGravity) (Variables|Default|GetTimePassed) (Variables|Default|GetTimePassed)))) false false))

(event EventBeginPlay
  (Variables|Default|SetLaunchPoint (Transformation|GetActorLocation)))

(fn ConstructionScript)