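; BP_CannonBall is a cannonball projectile that flies a ballistic arc, explodes on impact and carves into the ground.
; Tick computes displacement from launch speed, angle and gravity, then moves it with a swept SetActorLocation.
; A blocking hit spawns the explosion, draws a debug sphere and damages overlapping actors that have BP_HealthComponent.
; Two rings of line traces then supply angled planes that slice BP_GroundTile procedural meshes before the ball destroys itself.
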(event Custom|Setup
  (params (LaunchSpeed :type Float%20%28single-precision%29) (LaunchAngleInRad :type Float%20%28single-precision%29) (Gravity :type Float%20%28single-precision%29))
  (Variables|Default|SetSpeed LaunchSpeed)
  (Variables|Default|SetAngleInRad LaunchAngleInRad)
  (Variables|Default|SetGravity Gravity))

(event EventBeginPlay
  (Variables|Default|SetLaunchPoint (Transformation|GetActorLocation))
  (Variables|Status|SetDamageRadius (Variables|/Script/Engine.SphereComponent|GetSphereRadius (Variables|Default|GetDamageArea))))

(event EventTick
  (params (DeltaSeconds :type Float%20%28single-precision%29))
  (bind _returnvalue (Components|GetOwner))
  (bind (_x _y) (CallFunction|GetDisplacement))
  ;[1 1 1] Move the ball
  (Variables|Default|SetTimePassed (+ DeltaSeconds (Variables|Default|GetTimePassed)))
  (bind _sweephitresult (Transformation|SetActorLocation (+ (Variables|Default|GetLaunchPoint) (* (Transformation|GetActorForwardVector) _x) (* (Transformation|GetActorUpVector) _y)) true false))
  ;[1 1 1] Hit check
  (if (.bBlockingHit (Collision|BreakHitResult _sweephitresult))
    ;[1 1 1] Spawn Emitter (Explosion)
    (Effects|SpawnEmitteratLocation (Variables|Status|GetExplosionEmitter) (.ImpactPoint (Collision|BreakHitResult _sweephitresult)) "0, 0, 0" (Math|Conversions|ToVector(Float) (/ (Variables|Status|GetDamageRadius) 1e+02)))
    ;[1 1 1] Debugging the damage radius
    (Rendering|Debug|DrawDebugSphere (.ImpactPoint (Collision|BreakHitResult _sweephitresult)) (Variables|Status|GetDamageRadius) 12 "(R=1.000000,G=0.522653,B=0.119437,A=1.000000)" 1.0 3.0)
    ;[1 1 1] Apply damage on every actors with BP_HealthComp
    (for _array_element (Collision|GetOverlappingActors (Variables|Default|GetDamageArea) "/Script/Engine.Actor" :!class /Script/Engine.PrimitiveComponent)
      (if (Utilities|IsValid (Actor|GetComponentbyClass _array_element "/Game/Blueprints/BP_HealthComponent.BP_HealthComponent_C"))
        (Game|Damage|ApplyDamage _array_element (Variables|Status|GetDamage) (Game|GetInstigatorController _returnvalue) _returnvalue)))
    (Utilities|FlowControl|Sequence
      (:then_0
        ;[1 1 1] Gets points aligned in a circle on the ground
        (for _index (range 0 (Variables|Default|GetXLength))
          (Variables|Default|SetX _index)
          (bind _outhit (CallFunction|GetPointinCircle (Variables|Default|GetExplosionRadius) 2e+02))
          (Utilities|Array|Add (Variables|Default|GetOut%20Hit) _outhit)
          (bind _outhit_2 (CallFunction|GetPointinCircle (* (Variables|Default|GetExplosionRadius) 0.5) 4e+02))
          (Utilities|Array|Add (Variables|Default|GetOut%20Hit) _outhit_2))
        ;[1 1 1] Slicing the floor mesh with previously gotten points
        (for _array_element_2 (Variables|Default|GetOut%20Hit)
          (bind _asbp_ground_tile (Utilities|Casting|CastToBP_GroundTile (.HitActor (Collision|BreakHitResult _array_element_2))))
          (Class|KismetProceduralMeshLibrary|SliceProceduralMesh (Variables|/Game/Blueprints/SuperTest/BP_GroundTile.BP_GroundTile_C|GetProceduralMesh _asbp_ground_tile) (.ImpactPoint (Collision|BreakHitResult _array_element_2)) (Math|Vector|NegateVector (Math|Vector|Normalize (- (+ (Transformation|GetActorLocation) (* (.ImpactNormal (Collision|BreakHitResult _array_element_2)) (* (Math|Vector|VectorLength (- (Transformation|GetActorLocation) (.ImpactPoint (Collision|BreakHitResult _array_element_2)))) (Variables|Default|GetDepthWeight)))) (.ImpactPoint (Collision|BreakHitResult _array_element_2))))) false "UseLastSectionForCap" "/Engine/MaterialTemplates/VertexAnimation/AdvancedFlag.AdvancedFlag")))
      (:then_1
        (Actor|DestroyActor)))))

(fn ConstructionScript
  (Components|Sphere|SetSphereRadius (Variables|Default|GetDamageArea) (Variables|Status|GetDamageRadius) true))

(fn GetDisplacement
  (bind _timepassed (Variables|Default|GetTimePassed))
  (bind _output_get (Variables|Default|SetDisplacementX (* (* (Variables|Default|GetTimePassed) (Variables|Default|GetSpeed) (Math|Trig|Cos(Radians) (Variables|Default|GetAngleInRad))) 1e+02)))
  (bind _output_get_2 (Variables|Default|SetDisplacementY (* (- (* (Variables|Default|GetTimePassed) (Variables|Default|GetSpeed) (Math|Trig|Sin(Radians) (Variables|Default|GetAngleInRad))) (* 0.5 (Variables|Default|GetGravity) _timepassed _timepassed)) 1e+02)))
  (return _output_get _output_get_2))

(fn GetPointinCircle
  (params (Radius :type Float%20%28single-precision%29) (Range :type Float%20%28single-precision%29))
  (bind _returnvalue (Transformation|GetActorForwardVector))
  (bind _returnvalue_2 (Transformation|GetActorUpVector))
  (bind _returnvalue_3 (Transformation|GetActorLocation))
  (bind _x (Variables|Default|GetX))
  (bind _xlength (Variables|Default|GetXLength))
  (bind _returnvalue_4 (Math|Conversions|ToFloat(Integer) _x))
  (bind _returnvalue_5 (Math|Conversions|ToFloat(Integer) _xlength))
  (bind _returnvalue_6 (/ _returnvalue_4 _returnvalue_5))
  (bind _returnvalue_7 (* _returnvalue_6 3.6e+02))
  (bind _returnvalue_8 (Math|Vector|RotateVectorAroundAxis _returnvalue _returnvalue_7 _returnvalue_2))
  (bind _returnvalue_9 (* _returnvalue_8 Radius))
  (bind _returnvalue_10 (+ _returnvalue_9 _returnvalue_3))
  (bind _outhit (Collision|LineTraceByChannel (+ _returnvalue_10 (Math|Vector|MakeVector 0.0 0.0 Range)) (- _returnvalue_10 (Math|Vector|MakeVector 0.0 0.0 Range)) "TraceTypeQuery1" false 0 "ForOneFrame"))
  (return _outhit))