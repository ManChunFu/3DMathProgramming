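; BP_IKSolver2 is a procedurally animated four-legged IK walker with two-segment legs and a movable body.
; The construction script poses each leg toward its target via MovementT and offsets the body.
; Move runs one gait cycle, stepping diagonal leg pairs with a body shift between them.
; All legs share the LeftFront timeline, scaled by MoveSteps into UpdateInterp; older target-seeking and per-leg timeline chains are disconnected.
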(event Custom|NextLeg
  (bind (_direction _x _y _z) (Timeline|AnimatedCurveLeftFront PlayFromStart)
    (:Update
      (Class|IKSolver|UpdateInterp (Variables|Default|GetMoveTypes) (CallFunction|MoveStepsCalculation _x _y _z)))
    (:Finished
      (Variables|Default|SetbFirstTime true)
      (if (== (Variables|Default|GetLegOrder) 4) :!label _label
        (Variables|Default|SetLegOrder 0)
        (Variables|Default|SetMoveTypes "EMT_LeftFront")
        (Variables|Default|SetHasFinished false)
        (else
          (bind _result (Math|Integer|IncrementInt (Variables|Default|GetLegOrder))
            (:%20%20
              (if (Utilities|Enum|Equal(Enum) (CallFunction|SwitchLegs _result) "EMT_Body")
                (bind (_direction_2 _x_2 _y_2) (Timeline|AnimatedCurveBody PlayFromStart)
                  (:Update
                    (Class|IKSolver|UpdateInterp "EMT_Body" (CallFunction|MoveStepsCalculation _x_2 _y_2 0.0)))
                  (:Finished
                    (Variables|Default|SetbFirstTime true)
                    (goto _label)))
                (else
                  (CallFunction|NextLeg))))))))))

(event EventBeginPlay)

(event Collision|EventActorBeginOverlap
  (params (OtherActor :type Actor%20Object%20Reference)))

(event EventMove
  (if (not (Variables|Default|GetHasFinished))
    (Variables|Default|SetHasFinished true)
    (Utilities|FlowControl|Delay 0.5)
    (bind (_direction _x _y _z) (Timeline|AnimatedCurveLeftFront PlayFromStart)
      (:Update
        (Class|IKSolver|UpdateInterp (Variables|Default|GetMoveTypes) (CallFunction|MoveStepsCalculation _x _y _z)))
      (:Finished
        (Variables|Default|SetbFirstTime true)
        (if (== (Variables|Default|GetLegOrder) 4) :!label _label
          (Variables|Default|SetLegOrder 0)
          (Variables|Default|SetMoveTypes "EMT_LeftFront")
          (Variables|Default|SetHasFinished false)
          (else
            (bind _result (Math|Integer|IncrementInt (Variables|Default|GetLegOrder))
              (:%20%20
                (if (Utilities|Enum|Equal(Enum) (CallFunction|SwitchLegs _result) "EMT_Body")
                  (bind (_direction_2 _x_2 _y_2) (Timeline|AnimatedCurveBody PlayFromStart)
                    (:Update
                      (Class|IKSolver|UpdateInterp "EMT_Body" (CallFunction|MoveStepsCalculation _x_2 _y_2 0.0)))
                    (:Finished
                      (Variables|Default|SetbFirstTime true)
                      (goto _label)))
                  (else
                    (CallFunction|NextLeg)))))))))))

(fn ConstructionScript
  (Variables|Default|SetUpperLength 4e+01)
  (Class|IKSolver|MovementT (Variables|Default|GetUpperSegment) (Variables|Default|GetLowerSegment) (Variables|Default|GetEndPoint) (Variables|Default|GetJoint) (Variables|Default|GetLFTargetLocation))
  (Class|IKSolver|MovementT (Variables|Default|GetRBUpper) (Variables|Default|GetRBLower) (Variables|Default|GetRBEndPoint) (Variables|Default|GetRBJoint) (Variables|Default|GetRBTargetLocation))
  (Transformation|SetRelativeLocation (Variables|Default|GetBody) (+ (Variables|Default|GetBodyOffset) (Variables|Default|GetIKOrigin)) false false)
  (Class|IKSolver|MovementT (Variables|Default|GetRUpperSegment) (Variables|Default|GetRLowerSegment) (Variables|Default|GetREndPoint) (Variables|Default|GetRJoint) (Variables|Default|GetRFTargetLocation))
  (Class|IKSolver|MovementT (Variables|Default|GetLBUpper) (Variables|Default|GetLBLower) (Variables|Default|GetLBEndPoint) (Variables|Default|GetLBJoint) (Variables|Default|GetLBTargetLocation)))

(fn MoveStepsCalculation
  (params (X :type Float%20%28single-precision%29) (Y :type Float%20%28single-precision%29) (Z :type Float%20%28single-precision%29))
  (bind _movesteps (Variables|Default|GetMoveSteps))
  (return (Math|Vector|MakeVector (* X (.x _movesteps)) (* Y (.y _movesteps)) (* Z (.z _movesteps)))))

(fn SwitchLegs
  (params (legOrder :type Integer))
  (switch int legOrder
    (:0
      (bind _output_get (Variables|Default|SetMoveTypes "EMT_LeftFront"))
      (return _output_get))
    (:1
      (bind _output_get_2 (Variables|Default|SetMoveTypes "EMT_RightBehind"))
      (return _output_get_2))
    (:2
      (bind _output_get_3 (Variables|Default|SetMoveTypes "EMT_Body"))
      (return _output_get_3))
    (:3
      (bind _output_get_4 (Variables|Default|SetMoveTypes "EMT_RightFront"))
      (return _output_get_4))
    (:4
      (bind _output_get_5 (Variables|Default|SetMoveTypes "EMT_LeftBehind"))
      (return _output_get_5))))

(fn GetLegLocation
  (params (MoveType :type EMoveTypes%20Enum :default "EMT_LeftFront"))
  (switch Utilities|FlowControl|Switch|SwitchonEMoveTypes MoveType
    (:EMT_LeftFront
      (return (Variables|Default|GetLFTargetLocation)))
    (:EMT_LeftBehind
      (return (Variables|Default|GetLBTargetLocation)))
    (:EMT_Body
      (return (Variables|Default|GetIKOrigin)))
    (:EMT_RightFront
      (return (Variables|Default|GetRFTargetLocation)))
    (:EMT_RightBehind
      (return (Variables|Default|GetRBTargetLocation)))))

(fn GetLimbs
  (params (MoveType :type EMoveTypes%20Enum :default "EMT_LeftFront"))
  (switch Utilities|FlowControl|Switch|SwitchonEMoveTypes MoveType
    (:EMT_LeftFront
      (return (Variables|Default|GetUpperSegment) (Variables|Default|GetLowerSegment) (Variables|Default|GetEndPoint) (Variables|Default|GetJoint) (Variables|Default|GetLFTargetLocation) 0))
    (:EMT_LeftBehind
      (return (Variables|Default|GetLBUpper) (Variables|Default|GetLBLower) (Variables|Default|GetLBEndPoint) (Variables|Default|GetLBJoint) (Variables|Default|GetLBTargetLocation) 0))
    (:EMT_Body
      (return 0 0 0 0 "0, 0, 0" (Variables|Default|GetBody)))
    (:EMT_RightFront
      (return (Variables|Default|GetRUpperSegment) (Variables|Default|GetRLowerSegment) (Variables|Default|GetREndPoint) (Variables|Default|GetRJoint) (Variables|Default|GetRFTargetLocation) 0))
    (:EMT_RightBehind
      (return (Variables|Default|GetRBUpper) (Variables|Default|GetRBLower) (Variables|Default|GetRBEndPoint) (Variables|Default|GetRBJoint) (Variables|Default|GetRBTargetLocation) 0))))

(fn SetMovement)